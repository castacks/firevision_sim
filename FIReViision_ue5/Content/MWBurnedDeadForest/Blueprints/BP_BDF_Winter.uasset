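; BP_BDF_Winter is a weather actor for the Burned Dead Forest environment that builds up snow and keeps a particle effect around the player.
; On BeginPlay a timeline, rated by SnowAccumulationTime, ramps MW_SnowAmount in the MPC_BDF_Controller parameter collection up to SnowAmount and activates the particles.
; Tick eases the particle system toward the player pawn.
; The construction script also writes AutumnAmount to the collection, which the timeline update repeats.
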(event `self.ReceiveBeginPlay`
  (`TimelineComponent.SetPlayRate` (`self.SnowAccumulation`) (/ 1.0 (`self.SnowAccumulationTime`)))
  (bind (_direction _snowamount) (`Timeline|SnowAccumulation`)
    (:`Update`
      (`KismetMaterialLibrary.SetScalarParameterValue` "/Game/MWBurnedDeadForest/Materials/MASTER/Par/MPC_BDF_Controller.MPC_BDF_Controller" "MW_SnowAmount" (`KismetMathLibrary.Lerp` 0.0 (`self.SnowAmount`) _snowamount))
      (`KismetMaterialLibrary.SetScalarParameterValue` "/Game/MWBurnedDeadForest/Materials/MASTER/Par/MPC_BDF_Controller.MPC_BDF_Controller" "MW_AutumnAmount" (`self.AutumnAmount`))
      (`ActorComponent.SetActive` (`self.ParticleSystem`) true false))))

(event `self.ReceiveTick`
  (params (DeltaSeconds :type "Float (single-precision)"))
  (bind _particlesystem (`self.ParticleSystem`))
  (`SceneComponent.K2_SetWorldLocation` _particlesystem (`KismetMathLibrary.VInterpTo` (`SceneComponent.K2_GetComponentLocation` _particlesystem) (`self.K2_GetActorLocation` (`GameplayStatics.GetPlayerPawn` 0)) DeltaSeconds 1.0) false false))

(fn `UserConstructionScript`
  (`KismetMaterialLibrary.SetScalarParameterValue` "/Game/MWBurnedDeadForest/Materials/MASTER/Par/MPC_BDF_Controller.MPC_BDF_Controller" "MW_AutumnAmount" (`self.AutumnAmount`)))