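; BP_Human3 is a human pawn that wanders aimlessly by itself.
; On BeginPlay it starts RandomWalk, which uses AI MoveTo to reach a random reachable point near its current location and calls itself again on success or failure.
; Unconnected leftover nodes would apply a grayscale dynamic material to the mesh and add a post-process component, but they never run.
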(event `self.ReceiveBeginPlay`
  (`self.Random Walk`))

(event `Random Walk`
  ;[1 1 1] Random Walk Code
  (`|AIMoveTo` self (`NavigationSystemV1.K2_GetRandomReachablePointInRadius` (`self.K2_GetActorLocation`) 500.0 null null) null
    (:`OnSuccess`
      _)
    (:`OnFail`
      _))
  (`self.Random Walk`))

(fn `UserConstructionScript`)